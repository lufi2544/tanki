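; Player-controlled tank pawn Blueprint that drives, aims and fires through TankMovement and TankAiming components.
; On BeginPlay it passes the barrel and turret to the aiming component and both tracks to the movement component.
; Movement axes forward intent to TankMovement, and Shoot triggers Fire on TankAiming.
; Aim axes orbit the camera rig, applying yaw to an azimuth gimbal and pitch to the spring arm.
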(event EventBeginPlay
  (Class|TankAimingComponent|Initialise (Variables|Default|GetTankAiming) (Variables|Default|GetTankBarrel1) (Variables|Default|GetTankTurret))
  (Class|TankMovementComponent|Initialise (Variables|Default|GetTankMovement) (Variables|Default|GetTankTrackRight) (Variables|Default|GetTankTrackLeft)))

(event Input|ActionEvents|InputActionShoot
  (params (Key :type Key%20Structure :default "None"))
  (:Pressed
    (Class|TankAimingComponent|Fire (Variables|Default|GetTankAiming))))

(event Input|AxisEvents|InputAxisAimAzimuth
  (params (AxisValue :type Float%20%28single-precision%29))
  ;[1 1 1] Aim Input Binding
  (Transformation|AddLocalRotation (Variables|Default|GetAsimothGimble) (Math|Rotator|MakeRotator 0.0 0.0 AxisValue) false false))

(event Input|AxisEvents|InputAxisAimElevation
  (params (AxisValue :type Float%20%28single-precision%29))
  ;[1 1 1] Aim Input Binding
  (Transformation|AddLocalRotation (Variables|Default|GetSpringArm) (Math|Rotator|MakeRotator 0.0 AxisValue 0.0) false false))

(event Input|AxisEvents|InputAxisMoveForward/BAckwards
  (params (AxisValue :type Float%20%28single-precision%29))
  ;[1 1 1] Input Binidng
  (Class|TankMovementComponent|IntendMoveForward (Variables|Default|GetTankMovement) AxisValue))

(event Input|AxisEvents|InputAxisMoveSides
  (params (AxisValue :type Float%20%28single-precision%29))
  ;[1 1 1] Input Binidng
  (Class|TankMovementComponent|IntendMoveSides (Variables|Default|GetTankMovement) AxisValue))

(fn ConstructionScript)