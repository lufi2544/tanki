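; Mortar Blueprint that sets up a mortar's aiming and its health bar widget at the start of play.
; BeginPlay initialises the TankAiming component with the barrel and turret parts.
; It then casts the HealthWidget's user widget to HealthBar, passes itself in as the owning mortar and sets the bar's colour to light blue.
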(event EventBeginPlay
  (Class|TankAimingComponent|Initialise (Variables|Default|GetTankAiming) (Variables|Default|GetTankBarrel) (Variables|Default|GetTankTurret))
  (bind _ashealth_bar (Utilities|Casting|CastToHealthBar (UserInterface|GetUserWidgetObject (Variables|Default|GetHealthWidget))))
  (Variables|/Game/Widgets/HealthBar.HealthBar_C|SetMortar _ashealth_bar self)
  (Variables|/Game/Widgets/HealthBar.HealthBar_C|SetColor1 _ashealth_bar (Math|Color|SelectColor :A "(R=0.000000,G=0.674769,B=0.911458,A=1.000000)" :bPickA true)))

(fn ConstructionScript)